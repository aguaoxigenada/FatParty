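; BP_Archer is a player pawn Blueprint that can grab and release through a Grabber and shows a countdown HUD.
; Grab input routes through server events to multicasts that drive the Grabber and set a Holding flag.
; While Holding, Tick requests the holding montage from the server every frame.
; On possession it creates WBP_HUD, and a looping one-second timer feeds it TimeCounter from GS_Countdown.
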(event `InputAction|Grab`
  (params (Key :type "Key Structure"))
  (:`Pressed`
    (`self.Server_ActionGrab`))
  (:`Released`
    (`self.Server_ActionRelease`)))

(event `Server_ActionGrab`
  (`self.MulticastGrab`))

(event `Server_ActionRelease`
  (`self.MulticastRelease`))

(event `MulticastGrab`
  (`Grabber.Grab` (`self.Grabber`))
  (set `self.Holding` true))

(event `MulticastRelease`
  (`Grabber.Release` (`self.Grabber`))
  (set `self.Holding` false))

(event `self.ReceivePossessed`
  (params (NewController :type "Controller Object Reference"))
  (`self.AddUI_widget`))

(event `AddUI_widget`
  (bind _returnvalue (`|CreateWidget` "/Game/Blueprints/UI/WBP_HUD.WBP_HUD_C" (`GameplayStatics.GetPlayerController` 0)))
  (bind _output_get (set `self.Ref_UIWidget` _returnvalue))
  (`UserWidget.AddToViewport` _output_get 0)
  (`KismetSystemLibrary.K2_SetTimer` null "SetCounter" 1.0 true))

(event `self.ReceiveTick`
  (params (DeltaSeconds :type "Float (single-precision)"))
  (if (`self.Holding`)
    (`self.Server_PlayAnimation` "/Game/Assets/Animations/Archer/Animations/AM_Holding.AM_Holding")))

(fn `SetCounter`
  (bind _ref_uiwidget (`self.Ref_UIWidget`))
  (`/Engine/EditorBlueprintResources/StandardMacros.IsValid` _ref_uiwidget
    (:`Is Valid`
      (`HudWidget.UpdateTime` _ref_uiwidget (`/Game/Blueprints/GameMode/GS_Countdown.TimeCounter` (cast `/Game/Blueprints/GameMode/GS_Countdown` (`GameplayStatics.GetGameState`) :!pure true))))))

(fn `UserConstructionScript`)