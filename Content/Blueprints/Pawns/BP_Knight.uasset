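; Playable knight pawn with networked grab and release of objects, sword combat and a countdown HUD.
; Grab input goes through server events to multicasts driving the Grabber, while Tick replays a hold montage.
; Sword hits use a looping-timer line trace between weapon sockets, damaging FatPartyEnemy or DestructibleObject actors with particles.
; Tick also nudges movement back and forth with sweeps to smooth collisions with moving objects; possession creates the timer-updated HUD.
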(event `InputAction|Grab`
  (params (Key :type "Key Structure"))
  (:`Pressed`
    (`self.Server_ActionGrab`))
  (:`Released`
    (`self.Server_ActionRelease`)))

(event `Server_ActionGrab`
  (`self.MulticastGrab`))

(event `Server_ActionRelease`
  (`self.MulticastRelease`))

(event `MulticastGrab`
  (`Grabber.Grab` (`self.Grabber`))
  (set `self.Holding` true))

(event `self.ReceiveTick`
  (params (DeltaSeconds :type "Float (single-precision)"))
  (bind _returnvalue (`self.K2_GetActorRotation`))
  (bind _charactermovement (`self.CharacterMovement`))
  ;[1 1 1] Hacer un movimiento fluido del personaje al chocarse con objetos que tienen movimiento.
  (`MovementComponent.K2_MoveUpdatedComponent` _charactermovement (1.0 1.0 0.0) _returnvalue true false)
  (`MovementComponent.K2_MoveUpdatedComponent` _charactermovement (-1.0 -1.0 0.0) _returnvalue true false)
  (if (`self.Holding`)
    (`self.Server_PlayAnimation` "/Game/Assets/Animations/Knight/Run/AM_HoldingKnight.AM_HoldingKnight")))

(event `MulticastRelease`
  (`Grabber.Release` (`self.Grabber`))
  (set `self.Holding` false))

(event `TriggerLineTracer`
  (bind _returnvalue (`KismetSystemLibrary.K2_SetTimerDelegate` (delegate `AppliMultiLineTrace`) 0.01 true))
  (set `self.LineTracerTimer` _returnvalue))

(event `HitParticles`
  (`ActorComponent.Activate` (`self.HitWeapon`) true))

(event `AppliMultiLineTrace`
  (bind _weapon (`self.Weapon`))
  (bind _outhit (`KismetSystemLibrary.LineTraceSingle` (`SceneComponent.GetSocketLocation` _weapon "Start") (`SceneComponent.GetSocketLocation` _weapon "End") "TraceTypeQuery2"))
  (bind (_bblockinghit _binitialoverlap _time _distance _location _impactpoint _normal _impactnormal _physmat _hitactor) (`GameplayStatics.BreakHitResult` _outhit))
  (bind _asfat_party_enemy (cast `FatPartyEnemy` _hitactor)
    (:`then`
      (`GameplayStatics.ApplyDamage` _asfat_party_enemy 10.0)
      (`self.HitParticles`))
    (:`CastFailed`
      (bind _asdestructible_object (cast `DestructibleObject` _hitactor))
      (`GameplayStatics.ApplyDamage` _asdestructible_object 10.0)
      (`self.HitParticles`))))

(event `StopTriggerSword`
  (`KismetSystemLibrary.K2_ClearAndInvalidateTimerHandle` (`self.LineTracerTimer`)))

(event `self.ReceivePossessed`
  (params (NewController :type "Controller Object Reference"))
  (`self.AddUI_widget`))

(event `AddUI_widget`
  (bind _returnvalue (`|CreateWidget` "/Game/Blueprints/UI/WBP_HUD.WBP_HUD_C" (`GameplayStatics.GetPlayerController` 0)))
  (bind _output_get (set `self.REF_HudPlayer` _returnvalue))
  (`UserWidget.AddToViewport` _output_get 0)
  (`KismetSystemLibrary.K2_SetTimer` null "SetCounter" 1.0 true))

(fn `SetCounter`
  (bind _ref_hudplayer (`self.REF_HudPlayer`))
  (`/Engine/EditorBlueprintResources/StandardMacros.IsValid` _ref_hudplayer
    (:`Is Valid`
      (`HudWidget.UpdateTime` _ref_hudplayer (`/Game/Blueprints/GameMode/GS_Countdown.TimeCounter` (cast `/Game/Blueprints/GameMode/GS_Countdown` (`GameplayStatics.GetGameState`) :!pure true))))))

(fn `UserConstructionScript`)