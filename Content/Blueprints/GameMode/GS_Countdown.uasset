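; Countdown timer, apparently on the GameState, that decrements every second and shows the remaining time on the player's HUD.
; Server and clients tick locally; the server copies the count to replicated TimeChecker, whose OnRep corrects client drift and restarts the timer.
; On authority, a check on the counter also applies heavy damage to the owner.
; HUD updates go through a cached BP_Knight reference taken from player controller 0.
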(event `self.ReceiveBeginPlay`
  (bind _returnvalue (`KismetSystemLibrary.K2_SetTimer` null "DecreaseTimer" 1.0 true))
  (set `self.TH_Counter` _returnvalue))

(fn `DecreaseTimer`
  (bind _result (`/Engine/EditorBlueprintResources/StandardMacros.DecrementInt` (`self.TimeCounter`))
    (:`  `
      (`/Engine/EditorBlueprintResources/ActorMacros.Switch Has Authority`
        (:`Authority`
          (set `self.TimeChecker` _result)
          (`self.SetCounter`)
          (if (`KismetMathLibrary.Conv_IntToBool` (`self.TimeCounter`))
            ;[1 1 1] Medio raro, por ahi es mejor mandar un evento a todos los players.
            (`GameplayStatics.ApplyDamage` (`self.GetOwner`) 1000.0)))
        (:`Remote`
          (`self.SetCounter`))))))

(fn `GetTimerCounter`
  (returns (ActualTime :type Integer))
  (return (`self.TimeCounter`)))

(fn `OnRep_TimeChecker`
  (if (!= (`self.TimeChecker`) (`self.TimeCounter`))
    (set `self.TimeCounter` (`self.TimeChecker`))
    (`KismetSystemLibrary.K2_ClearAndInvalidateTimerHandle` (`self.TH_Counter`))
    (bind _returnvalue (`KismetSystemLibrary.K2_SetTimer` null "DecreaseTimer" 1.0 true))
    (set `self.TH_Counter` _returnvalue)
    (`self.SetCounter`)))

(fn `SetCounter`
  (bind _returnvalue (`Controller.K2_GetPawn` (`GameplayStatics.GetPlayerController` 0)))
  (bind _ref_hudplayer (`/Game/Blueprints/Pawns/BP_Knight.REF_HudPlayer` (`self.Ref_Char`)))
  (`/Engine/EditorBlueprintResources/StandardMacros.IsValid` (`self.Ref_Char`)
    (:`Is Valid`
      _)
    (:`Is Not Valid`
      (`/Engine/EditorBlueprintResources/StandardMacros.IsValid` _returnvalue
        (:`Is Valid`
          (bind _asbp_knight (cast `/Game/Blueprints/Pawns/BP_Knight` _returnvalue))
          (set `self.Ref_Char` _asbp_knight)))))
  (`/Engine/EditorBlueprintResources/StandardMacros.IsValid` _ref_hudplayer
    (:`Is Valid`
      (`HudWidget.UpdateTime` _ref_hudplayer (`self.TimeCounter`)))))

(fn `UserConstructionScript`)