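; Game state that runs a match countdown and tracks loading progress for a loading screen widget.
; A looping one-second timer decrements the counter and updates timer widgets, while the authority sets TimeChecker and conditionally damages the owner.
; TimeChecker's OnRep resyncs drifting clients and restarts their timer.
; Loading events queue percentages, update the widget image, and define a delay-driven recursive lerp for the percent text.
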(event `self.ReceiveBeginPlay`
  (bind _returnvalue (`KismetSystemLibrary.K2_SetTimer` null "DecreaseTimer" 1.0 true))
  (set `self.TH_Counter` _returnvalue))

(event `LoadTry_Event`
  (`self.LoadingEndedGS`))

(event `SetPercent`
  (params (PercentIn :type "Float (double-precision)") (LoadingWidget :type "/Game/Blueprints/UI/WBP_Loading Object Reference"))
  (if (`self.FirstTime`)
    (set `self.Loading Widget` LoadingWidget)
    (set `self.FirstTime` false))
  (bind _output_get (set `self.Percent` (* PercentIn 100.0)))
  (`KismetArrayLibrary.Array_Add` (`self.RecievedPercentages`) _output_get)
  (set `self.LerpFinished` false)
  (if (not (>= _output_get 100.0))
    (`/Game/Blueprints/UI/WBP_Loading.ChangeImage` (`self.Loading Widget`) (`self.Percent`))))

(event `LerpHappening`
  ;[1 1 1] Borrar luego
  (`KismetSystemLibrary.Delay` 0.05)
  (set `self.Alpha` (+ (`self.Alpha`) 0.1))
  (if (>= (`self.Alpha`) 1.0)
    (if (>= (`self.Percent`) 100.0)
      (set `self.LerpFinished` true)
      (else
        (set `self.Alpha` 0.0)
        (set `self.A` (`self.B`))
        (set `self.LerpFinished` true)))
    (else
      (set `TextBlock.Text` (`KismetTextLibrary.Conv_DoubleToText` (`KismetMathLibrary.Lerp` (`self.A`) (`self.B`) (`self.Alpha`)) "HalfToEven") (`/Game/Blueprints/UI/WBP_Loading.LoadingPercent` (`self.Loading Widget`)))
      (`self.LerpHappening`))))

(event `Query`
  (bind _recievedpercentages (`self.RecievedPercentages`))
  (bind _output_get (set `self.B` (`|GetArrayItem` _recievedpercentages)))
  (`KismetArrayLibrary.Array_RemoveItem` _recievedpercentages _output_get))

(fn `DecreaseTimer`
  (bind _result (`/Engine/EditorBlueprintResources/StandardMacros.DecrementInt` (`self.TimeCounter`))
    (:`  `
      (`/Engine/EditorBlueprintResources/ActorMacros.Switch Has Authority`
        (:`Authority`
          (set `self.TimeChecker` _result)
          (`self.SetCounter`)
          (if (`KismetMathLibrary.Conv_IntToBool` (`self.TimeCounter`))
            ;[1 1 1] Medio raro, por ahi es mejor mandar un evento a todos los players.
            (`GameplayStatics.ApplyDamage` (`self.GetOwner`) 1000.0)))
        (:`Remote`
          (`self.SetCounter`))))))

(fn `GetTimerCounter`
  (returns (ActualTime :type Integer))
  (return (`self.TimeCounter`)))

(fn `OnRep_Loading Widget`)

(fn `OnRep_LoadingEnded`)

(fn `OnRep_LoadTry`)

(fn `OnRep_NewVar`)

(fn `OnRep_TimeChecker`
  (if (!= (`self.TimeChecker`) (`self.TimeCounter`))
    (set `self.TimeCounter` (`self.TimeChecker`))
    (`KismetSystemLibrary.K2_ClearAndInvalidateTimerHandle` (`self.TH_Counter`))
    (bind _returnvalue (`KismetSystemLibrary.K2_SetTimer` null "DecreaseTimer" 1.0 true))
    (set `self.TH_Counter` _returnvalue)
    (`self.SetCounter`)))

(fn `SetCounter`
  (locals (NewLocalVar :type "Array of TimerWidget Object Reference"))
  (bind _foundwidgets (`WidgetBlueprintLibrary.GetAllWidgetsOfClass` "/Script/FatParty.TimerWidget"))
  (`TimerWidget.UpdateTime` _foundwidgets (`self.TimeCounter`)))

(fn `UserConstructionScript`)