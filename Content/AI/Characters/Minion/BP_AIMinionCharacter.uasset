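; BP_AIMinionCharacter is the AI minion character Blueprint, providing damage detection for its sword attack.
; TriggerLineTracer starts a fast looping timer that traces on the Camera channel between the Start and End sockets of WeaponMesh.
; Each trace applies a small fixed damage to the hit actor, with no filter against repeated hits, until StopTriggerSword clears the timer.
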(event `TriggerLineTracer`
  (bind _returnvalue (`KismetSystemLibrary.K2_SetTimerDelegate` (delegate `AppliMultiLineTrace`) 0.01 true))
  (set `self.MultiLineTracerTimer` _returnvalue))

(event `AppliMultiLineTrace`
  (bind _weaponmesh (`self.WeaponMesh`))
  (bind _outhit (`KismetSystemLibrary.LineTraceSingle` (`SceneComponent.GetSocketLocation` _weaponmesh "Start") (`SceneComponent.GetSocketLocation` _weaponmesh "End") "TraceTypeQuery2"))
  (`GameplayStatics.ApplyDamage` (`.HitActor` (`GameplayStatics.BreakHitResult` _outhit)) 2.0))

(event `StopTriggerSword`
  (`KismetSystemLibrary.K2_ClearAndInvalidateTimerHandle` (`self.MultiLineTracerTimer`)))

(fn `UserConstructionScript`)